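; BP_Train is a train Blueprint that moves a static mesh along a spline path.
; Tick calls Play on the MoveTrain timeline, whose TravelTrain track is scaled by the spline length to give a distance.
; Each timeline update places the mesh at that distance in world space and sets its relative rotation from the spline's local-space rotation.
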(event EventTick
  (params (DeltaSeconds :type Float%20%28single-precision%29))
  (bind _spline (Variables|Default|GetSpline))
  (bind _traveltrain (Timeline|MoveTrain Play)
    (:Update
      (Transformation|SetWorldLocation (Variables|Default|GetStaticMesh) (Spline|GetLocationatDistanceAlongSpline _spline (* _traveltrain (Spline|GetSplineLength (Variables|Default|GetSpline))) "World") false false)
      (Transformation|SetRelativeRotation (Variables|Default|GetStaticMesh) (Spline|GetRotationatDistanceAlongSpline _spline (* _traveltrain (Spline|GetSplineLength (Variables|Default|GetSpline))) "Local") false false))))

(fn ConstructionScript)