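; BP_Gear is a spinning pickup that the player collects by touching it.
; On Tick, the Cube mesh turns by a fixed yaw step each frame, so its spin speed depends on frame rate.
; When a ThirdPersonCharacter overlaps the Box, it increments that character's Collectable count and destroys itself.
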(event OnComponentBeginOverlap(Box)
  (params (OverlappedComponent :type Primitive%20Component%20Object%20Reference) (OtherActor :type Actor%20Object%20Reference) (OtherComp :type Primitive%20Component%20Object%20Reference) (OtherBodyIndex :type Integer) (bFromSweep :type Boolean) (SweepResult :type Hit%20Result%20Structure%20%28by%20ref%29))
  (bind _asthird_person_character (Utilities|Casting|CastToThirdPersonCharacter OtherActor))
  (Variables|/Game/ThirdPersonBP/Blueprints/ThirdPersonCharacter.ThirdPersonCharacter_C|SetCollectable _asthird_person_character (+ (Variables|/Game/ThirdPersonBP/Blueprints/ThirdPersonCharacter.ThirdPersonCharacter_C|GetCollectable _asthird_person_character) 1))
  (Actor|DestroyActor))

(event EventTick
  (params (DeltaSeconds :type Float%20%28single-precision%29))
  (bind _cube (Variables|Default|GetCube))
  (bind _relativerotation (Variables|/Script/Engine.SceneComponent|GetRelativeRotation _cube))
  (Transformation|SetRelativeRotation _cube (Math|Rotator|MakeRotator (.roll _relativerotation) (.pitch _relativerotation) (+ (.yaw _relativerotation) 2.0)) false false))

(fn ConstructionScript)